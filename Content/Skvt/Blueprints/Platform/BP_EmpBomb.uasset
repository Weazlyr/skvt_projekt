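; BP_EmpBomb is an interactable EMP device that the player triggers to hit a set of referenced lamps.
; Entering its sphere as a BP_SkvtBaseChar enables player input and shows a prompt, and leaving disables both.
; Pressing E once turns the spotlight red, hides the prompt, plays audio and calls EmpActivate on each lamp in LampsRef.
; The construction script applies the configurable spotlight settings and hides the prompt.
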(event OnComponentBeginOverlap(Sphere)
  (params (OverlappedComponent :type Primitive%20Component%20Object%20Reference) (OtherActor :type Actor%20Object%20Reference) (OtherComp :type Primitive%20Component%20Object%20Reference) (OtherBodyIndex :type Integer) (bFromSweep :type Boolean) (SweepResult :type Hit%20Result%20Structure%20%28by%20ref%29))
  ;[1 1 1] Enable/Disable input in sphere
  (Utilities|Casting|CastToBP_SkvtBaseChar OtherActor)
  (Input|EnableInput (Game|GetPlayerController 0))
  (Rendering|SetVisibility (Variables|Default|GetPressText) (not (Variables|Default|GetPressed?)) false))

(event OnComponentEndOverlap(Sphere)
  (params (OverlappedComponent :type Primitive%20Component%20Object%20Reference) (OtherActor :type Actor%20Object%20Reference) (OtherComp :type Primitive%20Component%20Object%20Reference) (OtherBodyIndex :type Integer))
  ;[1 1 1] Enable/Disable input in sphere
  (Input|DisableInput (Game|GetPlayerController 0))
  (Rendering|SetVisibility (Variables|Default|GetPressText) false false))

(event Custom|PlaySound
  (Audio|Components|Audio|Play (Variables|Default|GetAudio) 0.0))

(event Input|KeyboardEvents|E
  (params (Key :type Key%20Structure :default "None"))
  (:Pressed
    (if (not (Variables|Default|GetPressed?))
      (Rendering|Components|Light|SetLightColor (Variables|Default|GetSpotLight) "(R=1.000000,G=0.000000,B=0.021217,A=1.000000)" true)
      (Rendering|SetVisibility (Variables|Default|GetPressText) false false)
      (CallFunction|PlaySound)
      (for _array_element (Variables|Default|GetLampsRef)
        (Default|EmpActivate _array_element)
        (Variables|Default|SetPressed? true)))))

(fn ConstructionScript
  (bind _spotlight (Variables|Default|GetSpotLight))
  (Rendering|Components|Light|SetIntensity _spotlight (Variables|Default|GetIntensity))
  (Rendering|Components|Light|SetLightColor _spotlight (Variables|Default|GetNew%20Light%20Color) true)
  (Rendering|Lighting|SetInnerConeAngle _spotlight (Variables|Default|GetInner%20Cone%20Angle))
  (Rendering|Lighting|SetOuterConeAngle _spotlight (Variables|Default|GetOuter%20Cone%20Angle))
  (Rendering|SetVisibility (Variables|Default|GetPressText) false false))