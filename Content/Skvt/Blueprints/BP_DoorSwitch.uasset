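; BP_DoorSwitch is an interactable switch that remotely unlocks a referenced door for the female player character.
; Overlapping its InteractBox toggles an in-zone flag and the actor's input for player controller 0.
; IA_Interact sends RemoteUnlockDoorMessage to RemoteDoorRef while in zone, otherwise printing a failure string.
; On/off widget lookup functions exist but are not called here, and only the off lookup stores its result.
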(event OnComponentBeginOverlap(InteractBox)
  (params (OverlappedComponent :type Primitive%20Component%20Object%20Reference) (OtherActor :type Actor%20Object%20Reference) (OtherComp :type Primitive%20Component%20Object%20Reference) (OtherBodyIndex :type Integer) (bFromSweep :type Boolean) (SweepResult :type Hit%20Result%20Structure%20%28by%20ref%29))
  (Utilities|Casting|CastToBP_SkvtCharacterFemale OtherActor)
  (Input|EnableInput (Game|GetPlayerController 0))
  (Variables|Default|SetinZone? true))

(event OnComponentEndOverlap(InteractBox)
  (params (OverlappedComponent :type Primitive%20Component%20Object%20Reference) (OtherActor :type Actor%20Object%20Reference) (OtherComp :type Primitive%20Component%20Object%20Reference) (OtherBodyIndex :type Integer))
  (Utilities|Casting|CastToBP_SkvtCharacterFemale OtherActor)
  (Input|DisableInput (Game|GetPlayerController 0))
  (Variables|Default|SetinZone? false))

(event Input|EnhancedActionEvents|EnhancedInputActionIA_Interact
  (params (ActionValue :type Boolean) (ElapsedSeconds :type Float%20%28double-precision%29) (TriggeredSeconds :type Float%20%28double-precision%29) (InputAction :type Input%20Action%20Object%20Reference :default "/Game/Skvt/Characters/Input/Actions/IA_Interact.IA_Interact"))
  (if (Variables|Default|GetinZone?)
    (Class|BMIDoorRemote|RemoteUnlockDoor(Message) (Variables|Default|GetRemoteDoorRef))
    (else
      (Development|PrintString "Interface failed"))))

(fn ConstructionScript)

(fn GetonWidget
  (bind _foundwidgets (Widget|GetAllWidgetsOfClass "/Game/Skvt/UI/Widgets/Tutorial/WBP_TurnOn.WBP_TurnOn_C" true)))

(fn GetOffWidget
  (bind _foundwidgets (Widget|GetAllWidgetsOfClass "/Game/Skvt/UI/Widgets/Tutorial/WBP_TurnOff.WBP_TurnOff_C" true))
  (Variables|Default|SetWidgetOffRef (Utilities|Array|Get(acopy) _foundwidgets)))