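; Wall sconce light actor that can be knocked out by an EMP.
; The construction script applies its brightness, color and inner and outer cone angle variables to the spot-style SconceLight.
; EmpActivate waits briefly, sets the light intensity to zero and attaches a spark emitter to the lamp mesh, destroying the emitter after a further delay.
; Nothing in the graph restores the light afterward.
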(event EventEmpActivate
  (Utilities|FlowControl|Delay 4.0)
  (Rendering|Components|Light|SetIntensity (Variables|Default|GetSconceLight) 0.0)
  (bind _returnvalue (Effects|SpawnEmitterAttached "/Game/StarterContent/Particles/P_Sparks.P_Sparks" (Variables|Default|GetSM_Lamp_Wall) "None"))
  (Utilities|FlowControl|Delay 3.0)
  (Components|DestroyComponent _returnvalue))

(fn ConstructionScript
  (bind _sconcelight (Variables|Default|GetSconceLight))
  (Rendering|Components|Light|SetIntensity _sconcelight (Variables|Light|GetBrightness))
  (Rendering|Components|Light|SetLightColor _sconcelight (Variables|Light|GetColor) true)
  (Rendering|Lighting|SetInnerConeAngle _sconcelight (Variables|Light|GetInner%20Cone%20Angle))
  (Rendering|Lighting|SetOuterConeAngle _sconcelight (Variables|Light|GetOuter%20Cone%20Angle)))