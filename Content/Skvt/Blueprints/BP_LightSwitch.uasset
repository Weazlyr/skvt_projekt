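; BP_LightSwitch is an interactable switch that toggles a referenced light on and off.
; A sphere-trigger overlap flags the female player character and starts its sphere trace, while a separate box enables interact input.
; Interacting flips LightsOn, messages LightsRef, removes the current prompt widget and updates WidgetCheck.
; CreateWidget uses that flag to show a turn-on or turn-off prompt, but nothing here calls it.
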(event OnComponentEndOverlap(StartSphereTrace)
  (params (OverlappedComponent :type Primitive%20Component%20Object%20Reference) (OtherActor :type Actor%20Object%20Reference) (OtherComp :type Primitive%20Component%20Object%20Reference) (OtherBodyIndex :type Integer))
  (bind _asbp_skvt_character_female (Utilities|Casting|CastToBP_SkvtCharacterFemale OtherActor))
  (Variables|/Game/Skvt/Characters/BP_SkvtCharacterFemale.BP_SkvtCharacterFemale_C|SetEnteredZone _asbp_skvt_character_female false))

(event OnComponentBeginOverlap(StartSphereTrace)
  (params (OverlappedComponent :type Primitive%20Component%20Object%20Reference) (OtherActor :type Actor%20Object%20Reference) (OtherComp :type Primitive%20Component%20Object%20Reference) (OtherBodyIndex :type Integer) (bFromSweep :type Boolean) (SweepResult :type Hit%20Result%20Structure%20%28by%20ref%29))
  (bind _asbp_skvt_character_female (Utilities|Casting|CastToBP_SkvtCharacterFemale OtherActor))
  (Variables|/Game/Skvt/Characters/BP_SkvtCharacterFemale.BP_SkvtCharacterFemale_C|SetEnteredZone _asbp_skvt_character_female true)
  (Default|TriggerSphereTrace _asbp_skvt_character_female))

(event OnComponentBeginOverlap(InteractBox)
  (params (OverlappedComponent :type Primitive%20Component%20Object%20Reference) (OtherActor :type Actor%20Object%20Reference) (OtherComp :type Primitive%20Component%20Object%20Reference) (OtherBodyIndex :type Integer) (bFromSweep :type Boolean) (SweepResult :type Hit%20Result%20Structure%20%28by%20ref%29))
  (Utilities|Casting|CastToBP_SkvtCharacterFemale OtherActor)
  (Input|EnableInput (Game|GetPlayerController 0)))

(event OnComponentEndOverlap(InteractBox)
  (params (OverlappedComponent :type Primitive%20Component%20Object%20Reference) (OtherActor :type Actor%20Object%20Reference) (OtherComp :type Primitive%20Component%20Object%20Reference) (OtherBodyIndex :type Integer))
  (Utilities|Casting|CastToBP_SkvtCharacterFemale OtherActor)
  (Input|DisableInput (Game|GetPlayerController 0)))

(event Custom|CreateWidget
  (if (Variables|Default|GetWidgetCheck)
    (bind _returnvalue (UserInterface|CreateWidget "/Game/Skvt/UI/Widgets/Tutorial/WBP_TurnOff.WBP_TurnOff_C"))
    (bind _output_get (Variables|Default|SetWidgetOffRef _returnvalue))
    (UserInterface|Viewport|AddtoViewport _output_get 0)
    (else
      (bind _returnvalue_2 (UserInterface|CreateWidget "/Game/Skvt/UI/Widgets/Tutorial/WBP_TurnOn.WBP_TurnOn_C"))
      (bind _output_get_2 (Variables|Default|SetWidgetOnRef _returnvalue_2))
      (UserInterface|Viewport|AddtoViewport _output_get_2 0))))

(event Input|EnhancedActionEvents|EnhancedInputActionIA_Interact
  (params (ActionValue :type Boolean) (ElapsedSeconds :type Float%20%28double-precision%29) (TriggeredSeconds :type Float%20%28double-precision%29) (InputAction :type Input%20Action%20Object%20Reference :default "/Game/Skvt/Characters/Input/Actions/IA_Interact.IA_Interact"))
  (bind _lightsref (Variables|Default|GetLightsRef))
  (if (Variables|Default|GetLightsOn?)
    (Variables|Default|SetLightsOn? false)
    (Class|BMILight|LightSwitchOff(Message) _lightsref)
    (Utilities|IsValid "/Game/Skvt/UI/Widgets/Tutorial/WBP_TurnOff.WBP_TurnOff"
      (:Is%20Valid
        (Widget|RemovefromParent (Variables|Default|GetWidgetOffRef))
        (Variables|Default|SetWidgetCheck false)))
    (else
      (Variables|Default|SetLightsOn? true)
      (Class|BMILight|LightSwitchon(Message) _lightsref)
      (Utilities|IsValid "/Game/Skvt/UI/Widgets/Tutorial/WBP_TurnOn.WBP_TurnOn"
        (:Is%20Valid
          (Widget|RemovefromParent (Variables|Default|GetWidgetOnRef))
          (Variables|Default|SetWidgetCheck true))))))

(fn ConstructionScript)

(fn GetonWidget
  (bind _foundwidgets (Widget|GetAllWidgetsOfClass "/Game/Skvt/UI/Widgets/Tutorial/WBP_TurnOn.WBP_TurnOn_C" true))
  (Variables|Default|SetWidgetOnRef (Utilities|Array|Get(acopy) _foundwidgets)))

(fn GetOffWidget
  (bind _foundwidgets (Widget|GetAllWidgetsOfClass "/Game/Skvt/UI/Widgets/Tutorial/WBP_TurnOff.WBP_TurnOff_C" true))
  (Variables|Default|SetWidgetOffRef (Utilities|Array|Get(acopy) _foundwidgets)))