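; BP_Door is an interactable swinging door that the player opens and closes with the Interact input.
; A Box trigger enables input while a BP_SkvtBaseChar overlaps it and disables it on exit.
; Each press flips between playing and reversing a timeline that sets the door's yaw.
; The timeline update also removes the tutorial's interact widget through TutorialRef.
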(event OnComponentBeginOverlap(Box)
  (params (OverlappedComponent :type Primitive%20Component%20Object%20Reference) (OtherActor :type Actor%20Object%20Reference) (OtherComp :type Primitive%20Component%20Object%20Reference) (OtherBodyIndex :type Integer) (bFromSweep :type Boolean) (SweepResult :type Hit%20Result%20Structure%20%28by%20ref%29))
  (Utilities|Casting|CastToBP_SkvtBaseChar OtherActor)
  (Input|EnableInput (Game|GetPlayerController 0)))

(event OnComponentEndOverlap(Box)
  (params (OverlappedComponent :type Primitive%20Component%20Object%20Reference) (OtherActor :type Actor%20Object%20Reference) (OtherComp :type Primitive%20Component%20Object%20Reference) (OtherBodyIndex :type Integer))
  (Utilities|Casting|CastToBP_SkvtBaseChar OtherActor)
  (Input|DisableInput (Game|GetPlayerController 0)))

(event Input|EnhancedActionEvents|EnhancedInputActionIA_Interact
  (params (ActionValue :type Boolean) (ElapsedSeconds :type Float%20%28double-precision%29) (TriggeredSeconds :type Float%20%28double-precision%29) (InputAction :type Input%20Action%20Object%20Reference :default "/Game/Skvt/Characters/Input/Actions/IA_Interact.IA_Interact"))
  (Utilities|FlowControl|FlipFlop
    (:A
      (bind _rotation (Timeline|DoorAnimation PlayFromStart)
        (:Update
          (Transformation|SetRelativeRotation (Variables|Default|GetDoor) (Math|Rotator|MakeRotator 0.0 0.0 _rotation) false false)
          (Widget|RemovefromParent (Variables|/Game/Skvt/Blueprints/BP_TutorialInteract.BP_TutorialInteract_C|GetTutorialInteractWidget (Variables|Default|GetTutorialRef))))))
    (:B
      (Timeline|DoorAnimation ReverseFromEnd))))

(event EventBeginPlay)

(event Collision|EventActorBeginOverlap
  (params (OtherActor :type Actor%20Object%20Reference)))

(event EventTick
  (params (DeltaSeconds :type Float%20%28single-precision%29)))

(fn ConstructionScript)