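; Female character Blueprint that detects when the character's view falls on a light switch and opens that switch's widget.
; While EnteredZone is true, TriggerSphereTrace re-arms a half-second looping timer and sphere-traces on Visibility between two view arrows, with debug drawing.
; A hit is matched by the display name BP_LightSwitch, then CreateWidget is called on the switch returned by GetActorOfClass, rather than the hit actor.
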(event Custom|TriggerSphereTrace
  (if (Variables|Default|GetEnteredZone)
    (Utilities|Time|SetTimerbyEvent (delegate Custom|TriggerSphereTrace) 0.5 (Variables|Default|GetEnteredZone))
    (bind (_outhit _returnvalue) (Collision|SphereTraceByChannel (Transformation|GetWorldLocation (Variables|Default|GetViewArrowStart)) (Transformation|GetWorldLocation (Variables|Default|GetViewArrowEnd)) 5e+01 "TraceTypeQuery1" false 0 "ForDuration" true "(R=1.000000,G=0.000000,B=0.000000,A=1.000000)" "(R=0.000000,G=1.000000,B=0.000000,A=1.000000)" 2.0))
    (if _returnvalue
      (if (Utilities|Enum|Equal(Enum) (Utilities|GetDisplayName (.HitActor (Collision|BreakHitResult _outhit))) "BP_LightSwitch")
        (bind _returnvalue_2 (Actor|GetActorOfClass "/Game/Skvt/Blueprints/BP_LightSwitch.BP_LightSwitch_C"))
        (Default|CreateWidget _returnvalue_2)))))

(fn ConstructionScript)