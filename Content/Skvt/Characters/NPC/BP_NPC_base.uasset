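; BP_NPC_base is a base NPC character Blueprint that handles taking damage and dying.
; Any damage is passed to the health component and plays a punch hit-reaction montage.
; When the health component signals death, movement is disabled, the mesh switches to ragdoll physics, and the actor is destroyed after a short timer.
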(event OnDeath(Health_Component)
  (Pawn|Components|CharacterMovement|DisableMovement (Variables|Character|GetCharacterMovement))
  (Physics|SetSimulatePhysics (Variables|Character|GetMesh) true)
  (Utilities|Time|SetTimerbyEvent (delegate Custom|FinalizeDeath) 5.0))

(event Custom|FinalizeDeath
  (Actor|DestroyActor))

(event Game|Damage|EventAnyDamage
  (params (Damage :type Float%20%28single-precision%29) (DamageType :type Damage%20Type%20Object%20Reference) (InstigatedBy :type Controller%20Object%20Reference) (DamageCauser :type Actor%20Object%20Reference))
  (Default|ProcessDamage (Variables|Default|GetHealth_Component) Damage)
  (Animation|PlayAnimMontage "/Game/Skvt/Characters/Animations/Attacks/AM_Hit_punch.AM_Hit_punch" 1.0 "None"))

(fn ConstructionScript)