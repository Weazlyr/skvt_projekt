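; Player controller that handles character swapping, the pause main menu and a movement tutorial prompt.
; On BeginPlay it adds the default and swap Enhanced Input contexts and starts a timer that shows the move tutorial; move input cancels the timer or removes the widget.
; Swap input possesses the next BP_SkvtBaseChar in the actor list, wrapping to the first.
; The menu toggle creates or removes the widget, switching input mode, cursor and pause.
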(event Custom|ShowMoveTutorial
  (bind _returnvalue (UserInterface|CreateWidget "/Game/Skvt/UI/Widgets/Tutorial/WBP_MoveTutorial.WBP_MoveTutorial_C" self))
  (bind _output_get (Variables|Tutorial|SetMoveTutorialWidget _returnvalue))
  (UserInterface|Viewport|AddtoViewport _output_get 0))

(event Custom|HideMoveTutorial
  (Widget|RemovefromParent (Variables|Tutorial|GetMoveTutorialWidget)))

(event Input|EnhancedActionEvents|EnhancedInputActionIA_Swap
  (params (ActionValue :type Boolean) (ElapsedSeconds :type Float%20%28double-precision%29) (TriggeredSeconds :type Float%20%28double-precision%29) (InputAction :type Input%20Action%20Object%20Reference :default "/Game/Skvt/Characters/Input/Actions/IA_Swap.IA_Swap"))
  (bind _outactors (Actor|GetAllActorsOfClass "/Game/Skvt/Characters/BP_SkvtBaseChar.BP_SkvtBaseChar_C"))
  (Pawn|Possess (CallFunction|SelectCharactertoPossess _outactors)))

(event Input|EnhancedActionEvents|EnhancedInputActionIA_OpenMainMenu
  (params (ActionValue :type Boolean) (ElapsedSeconds :type Float%20%28double-precision%29) (TriggeredSeconds :type Float%20%28double-precision%29) (InputAction :type Input%20Action%20Object%20Reference :default "/Game/Skvt/UI/Input/IA_OpenMainMenu.IA_OpenMainMenu"))
  ;[0.526 0.526 0.526] Main Menu
  (Utilities|IsValid (Variables|Default|GetMainMenuWidget)
    (:Is%20Valid
      (CallFunction|CloseMainMenu))
    (:Is%20Not%20Valid
      (CallFunction|OpenMainMenu))))

(event Input|EnhancedActionEvents|EnhancedInputActionIA_Move
  (params (ActionValue :type Vector%202D%20Structure) (ElapsedSeconds :type Float%20%28double-precision%29) (TriggeredSeconds :type Float%20%28double-precision%29) (InputAction :type Input%20Action%20Object%20Reference :default "/Game/ThirdPerson/Input/Actions/IA_Move.IA_Move"))
  (Utilities|IsValid (Variables|Tutorial|GetMoveTutorialWidget)
    (:Is%20Valid
      (CallFunction|HideMoveTutorial))
    (:Is%20Not%20Valid
      (Utilities|Time|ClearandInvalidateTimerbyHandle (Variables|Tutorial|GetMoveTutorialTimer)))))

(event EventBeginPlay
  (CallFunction|AddInputMappings)
  (bind _returnvalue (Utilities|Time|SetTimerbyEvent (delegate Custom|ShowMoveTutorial) (Variables|Tutorial|GetTime)))
  (Variables|Tutorial|SetMoveTutorialTimer _returnvalue))

(fn ConstructionScript)

(fn SelectCharactertoPossess
  (params (Characters :type Array%20of%20Pawn%20Object%20References))
  (bind _returnvalue (Game|Player|GetPlayerPawn 0))
  (bind _returnvalue_2 (Utilities|Array|FindItem Characters _returnvalue))
  (bind _returnvalue_3 (+ _returnvalue_2 1))
  (if (< _returnvalue_3 (Utilities|Array|Length Characters))
    (return (Utilities|Array|Get(acopy) Characters _returnvalue_3))
    (else
      (return (Utilities|Array|Get(acopy) Characters)))))

(fn OpenMainMenu
  (bind _returnvalue (UserInterface|CreateWidget "/Game/Skvt/UI/Widgets/Menu/WBP_MainMenu.WBP_MainMenu_C" self))
  (bind _output_get (Variables|Default|SetMainMenuWidget _returnvalue))
  (UserInterface|Viewport|AddtoViewport _output_get 0)
  (Input|SetInputModeGameandUI self 0 "DoNotLock" true false)
  (Variables|Default|SetbShowMouseCursor true)
  (Game|SetGamePaused true))

(fn CloseMainMenu
  (Widget|RemovefromParent (Variables|Default|GetMainMenuWidget))
  (Variables|Default|SetMainMenuWidget 0)
  (Input|SetInputModeGameOnly self false)
  (Variables|Default|SetbShowMouseCursor false)
  (Game|SetGamePaused false))

(fn AddInputMappings
  (bind _self self)
  (bind _returnvalue (PlayerController|LocalPlayerSubsystems|GetEnhancedInputLocalPlayerSubsystem _self))
  (Utilities|IsValid _returnvalue
    (:Is%20Valid
      (Input|AddMappingContext _returnvalue "/Game/ThirdPerson/Input/IMC_Default.IMC_Default" 0 "(bIgnoreAllPressedKeysUntilRelease=True,bForceImmediately=False,bNotifyUserSettings=False)")
      (Input|AddMappingContext _returnvalue "/Game/Skvt/Characters/Input/IMC_SwapPawn.IMC_SwapPawn" 0 "(bIgnoreAllPressedKeysUntilRelease=True,bForceImmediately=False,bNotifyUserSettings=False)"))))